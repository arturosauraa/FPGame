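; BP_Key is a key pickup that gives the interacting player its KeyChannel through AddKey, then destroys itself.
; On BeginPlay, each key creates its own Interact_Prompt_Widget and adds it to the viewport.
; BoxTrigger overlaps with BP_FirstPersonCharacter show and hide the grab prompt, while the pickup itself runs from the OnInteraction event.
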(event `/Game/FlashLight/2FlashLight/BPI_Item.OnInteraction`
  (params (Player :type "/Game/FirstPerson/Blueprints/BP_FirstPersonCharacter Object Reference"))
  ;[1 1 1] Grab Key
  (`/Engine/EditorBlueprintResources/StandardMacros.IsValid` Player
    (:`Is Valid`
      (`/Game/FirstPerson/Blueprints/BP_FirstPersonCharacter.AddKey` Player (`self.KeyChannel`))
      (`self.K2_DestroyActor`))))

(event `self.ReceiveBeginPlay`
  ;[1 1 1] Show Text to grab Key
  (bind _returnvalue (`|CreateWidget` "/Game/Widgets/Interact_Prompt_Widget.Interact_Prompt_Widget_C"))
  (`UserWidget.AddToViewport` _returnvalue 0)
  (set `self.InteractWidget` _returnvalue))

(event `self.BoxTrigger.OnComponentBeginOverlap`
  (params (OverlappedComponent :type "PrimitiveComponent Object Reference") (OtherActor :type "Actor Object Reference") (OtherComp :type "PrimitiveComponent Object Reference") (OtherBodyIndex :type Integer) (bFromSweep :type Boolean) (SweepResult :type "HitResult Structure (by ref)"))
  ;[1 1 1] Show Text to grab Key
  (cast `/Game/FirstPerson/Blueprints/BP_FirstPersonCharacter` OtherActor)
  (if true
    (`/Game/Widgets/Interact_Prompt_Widget.GrabAnObject` (`self.InteractWidget`))))

(event `self.BoxTrigger.OnComponentEndOverlap`
  (params (OverlappedComponent :type "PrimitiveComponent Object Reference") (OtherActor :type "Actor Object Reference") (OtherComp :type "PrimitiveComponent Object Reference") (OtherBodyIndex :type Integer))
  ;[1 1 1] Show Text to grab Key
  (cast `/Game/FirstPerson/Blueprints/BP_FirstPersonCharacter` OtherActor)
  (if true
    (`/Game/Widgets/Interact_Prompt_Widget.HideTextObject` (`self.InteractWidget`))))

(fn `UserConstructionScript`)