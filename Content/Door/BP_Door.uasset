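; BP_Door is a keyed door that a player opens or closes by interacting while holding a key for its KeyChannel.
; OnInteraction checks the key and toggles Open and Close, which play or reverse a timeline that rotates the door's yaw.
; On BeginPlay it creates two widgets, and a box trigger shows either the interact or no-key prompt to BP_FirstPersonCharacter, removing it on exit.
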(event `/Game/FlashLight/BPI_Item.OnInteraction`
  (params (Player :type "/Game/FirstPerson/Blueprints/BP_FirstPersonCharacter Object Reference"))
  (`/Engine/EditorBlueprintResources/StandardMacros.IsValid` Player
    (:`Is Valid`
      (if (`/Game/FirstPerson/Blueprints/BP_FirstPersonCharacter.HasKey?` Player (`self.KeyChannel`))
        (if (`self.Open?`)
          (`self.Close`)
          (else
            (`self.Open`)))))))

(event `Open`
  (set `self.Open?` true)
  (bind (_direction _doorrotation) (`Timeline|RotateDoorTimeline` :!label _label)
    (:`Update`
      (`SceneComponent.K2_SetRelativeRotation` (`self.Door`) (`KismetMathLibrary.MakeRotator` 0.0 0.0 _doorrotation) false false))))

(event `Close`
  (set `self.Open?` false)
  (goto _label :!via `Reverse`))

(event `self.ReceiveBeginPlay`
  ;[1 1 1] Show text near door
  (bind _returnvalue (`|CreateWidget` "/Game/Widgets/Interact_Prompt_Widget.Interact_Prompt_Widget_C"))
  (set `self.InteractPrompt` _returnvalue)
  (bind _returnvalue_2 (`|CreateWidget` "/Game/Widgets/NoKeyforDoor_Widget.NoKeyforDoor_Widget_C"))
  (set `self.NoKeyForDoorPrompt` _returnvalue_2))

(event `self.Box.OnComponentBeginOverlap`
  (params (OverlappedComponent :type "PrimitiveComponent Object Reference") (OtherActor :type "Actor Object Reference") (OtherComp :type "PrimitiveComponent Object Reference") (OtherBodyIndex :type Integer) (bFromSweep :type Boolean) (SweepResult :type "HitResult Structure (by ref)"))
  ;[1 1 1] Show text near door
  (bind _asbp_first_person_character (cast `/Game/FirstPerson/Blueprints/BP_FirstPersonCharacter` OtherActor))
  (if (`/Game/FirstPerson/Blueprints/BP_FirstPersonCharacter.HasKey?` _asbp_first_person_character (`self.KeyChannel`))
    (`UserWidget.AddToViewport` (`self.InteractPrompt`) 0)
    (else
      (`UserWidget.AddToViewport` (`self.NoKeyForDoorPrompt`) 0))))

(event `self.Box.OnComponentEndOverlap`
  (params (OverlappedComponent :type "PrimitiveComponent Object Reference") (OtherActor :type "Actor Object Reference") (OtherComp :type "PrimitiveComponent Object Reference") (OtherBodyIndex :type Integer))
  ;[1 1 1] Show text near door
  (bind _asbp_first_person_character (cast `/Game/FirstPerson/Blueprints/BP_FirstPersonCharacter` OtherActor))
  (if (`/Game/FirstPerson/Blueprints/BP_FirstPersonCharacter.HasKey?` _asbp_first_person_character (`self.KeyChannel`))
    (`Widget.RemoveFromParent` (`self.InteractPrompt`))
    (else
      (`Widget.RemoveFromParent` (`self.NoKeyForDoorPrompt`)))))

(fn `UserConstructionScript`)