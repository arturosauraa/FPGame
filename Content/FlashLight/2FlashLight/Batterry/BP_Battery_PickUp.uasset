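; BP_Battery_PickUp is an interactable battery pickup for the first-person player's flashlight.
; It caches the BP_FirstPersonCharacter on BeginPlay.
; On interaction, after a short delay, it adds a spare refill to that cached character, or fully recharges the battery instead when charge is nearly empty.
; It then destroys itself, with debug prints reporting the pickup and refill count.
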(event `self.ReceiveBeginPlay`
  ;[1 1 1] Player Casting
  (bind _asbp_first_person_character (cast `/Game/FirstPerson/Blueprints/BP_FirstPersonCharacter` (`GameplayStatics.GetPlayerCharacter` 0)))
  (set `self.Player Character` _asbp_first_person_character))

(event `/Game/FlashLight/2FlashLight/BPI_Item.OnInteraction`
  (params (Player :type "/Game/FirstPerson/Blueprints/BP_FirstPersonCharacter Object Reference"))
  (bind _player_character (`self.Player Character`))
  ;[1 1 1] Battery PickUp
  (`/Engine/EditorBlueprintResources/StandardMacros.IsValid` Player
    (:`Is Valid`
      (`KismetSystemLibrary.PrintString` "Item Picked")
      (`KismetSystemLibrary.Delay` 0.2)
      (if (>= (`/Game/FirstPerson/Blueprints/BP_FirstPersonCharacter.BatteryAmount` (`self.Player Character`)) 5)
        (bind _output_get (set `/Game/FirstPerson/Blueprints/BP_FirstPersonCharacter.BatteryRefill` (+ (`/Game/FirstPerson/Blueprints/BP_FirstPersonCharacter.BatteryRefill` _player_character) 1) _player_character))
        (else
          (set `/Game/FirstPerson/Blueprints/BP_FirstPersonCharacter.BatteryAmount` 100 (`self.Player Character`))))
      (`self.K2_DestroyActor`)
      (`KismetSystemLibrary.PrintString` (`KismetStringLibrary.Conv_IntToString` _output_get)))))

(fn `UserConstructionScript`)